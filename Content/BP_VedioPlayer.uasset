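; Actor that plays a video on a sphere mesh using an FFmpeg video player component.
; On BeginPlay it creates a dynamic instance of a test material on the sphere and starts playback of the video named by an enum variable.
; If playback starts, the player's video texture is fed into the material's texture parameter.
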(event Collision|EventActorBeginOverlap
  (params (OtherActor :type Actor%20Object%20Reference)))

(event EventTick
  (params (DeltaSeconds :type Float%20%28single-precision%29)))

(event EventBeginPlay
  (bind _ffmpegvideoplayer (Variables|Default|GetFfmpegVideoPlayer))
  (bind _returnvalue (Rendering|Material|CreateDynamicMaterialInstance (Variables|Default|GetSphere) 0 "/Game/MA_TEST.MA_TEST" "None" :!class /Script/Engine.PrimitiveComponent))
  (Variables|Default|SetMateria_Ins _returnvalue)
  (bind _returnvalue_2 (Class|FfmpegVideoPlayer|StartVideoPlayback _ffmpegvideoplayer (Utilities|String|EnumtoString (Variables|Default|GetEnum_video))))
  (if _returnvalue_2
    (Rendering|Material|SetTextureParameterValue (Variables|Default|GetMateria_Ins) "Param" (Class|FfmpegVideoPlayer|GetVideoTexture _ffmpegvideoplayer))))

(fn ConstructionScript)